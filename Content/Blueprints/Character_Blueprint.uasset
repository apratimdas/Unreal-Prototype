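; Player character for an on-rails track game that auto-advances along a spline, collecting items and jumping off ramps.
; Tick sets position and rotation from spline distance, adding sideways offset from touch or A/D input and timeline-driven jump height.
; Spline ends and fork triggers switch tracks through TrackManager's spline list.
; It also handles multiplier scoring with decay, a pause menu, collectible spawning and a creative-mode toggle that disables collection.
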(event Custom|tick4
  ;[1 1 1] Multiplier
  (Utilities|FlowControl|Delay 0.2)
  (bind _output_get (Variables|Default|SetMultiplierScore (Math|Integer|Clamp(Integer) (- (Variables|Default|GetMultiplierScore) 1) -1 100)))
  (if (> (Variables|Default|GetMultiplier) 1)
    (if (< _output_get 0)
      (Variables|Default|SetMultiplier (Math|Integer|Clamp(Integer) (- (Variables|Default|GetMultiplier) 1) 1 5))
      (Variables|Default|SetMultiplierScore (+ (Variables|Default|GetMultiplierScore) 100)))))

(event Custom|tick3
  (bind _returnvalue (Utilities|Time|GetWorldDeltaSeconds))
  (bind _returnvalue_2 (Game|GetPlayerController 0))
  (bind _spline_tangent (Variables|Default|GetSpline%20Tangent))
  (bind _sizex (HUD|GetViewportSize _returnvalue_2))
  (bind _returnvalue_3 (Math|Conversions|ToFloat(Integer) _sizex))
  (bind _returnvalue_4 (/ _returnvalue_3 2.0))
  ;[1 1 1] Test Touch Input
  (if (Variables|Default|GetCanMove)
    (Variables|Default|SetMiddlePoint _returnvalue_4)
    (Variables|Default|SetFingerXPos (.X (Math|Vector|BreakVector (stale Input|TouchEvents|InputTouch Location))))
    (Variables|Default|SetResult (* (- (Variables|Default|GetFingerXPos) (Variables|Default|GetMiddlePoint)) (Variables|Default|GetCharacterSideMovementSpeed)))
    (Math|Float|CompareFloat (.X (Math|Vector|BreakVector (stale Input|TouchEvents|InputTouch Location))) _returnvalue_4
      (:>
        (Math|Float|CompareFloat (Variables|Default|GetWidth%20Along%20Spline) 7e+02
          (:<
            (Variables|Default|SetWidth%20Along%20Spline (+ (Variables|Default|GetWidth%20Along%20Spline) (* (Variables|Default|GetResult) (Utilities|Time|GetWorldDeltaSeconds))))
            (Transformation|SetActorLocation (+ (* _spline_tangent (* _returnvalue (Variables|Default|GetResult))) (Transformation|GetActorLocation)) false false))))
      (:<
        (Math|Float|CompareFloat (Variables|Default|GetWidth%20Along%20Spline) -7e+02
          (:>
            (Variables|Default|SetWidth%20Along%20Spline (+ (Variables|Default|GetWidth%20Along%20Spline) (* (Variables|Default|GetResult) (Utilities|Time|GetWorldDeltaSeconds))))
            (Transformation|SetActorLocation (+ (Transformation|GetActorLocation) (* _spline_tangent (* (Variables|Default|GetResult) _returnvalue))) false false)))))))

(event Custom|DoJump
  ;[1 1 1] Jumping
  (Variables|Default|SetIsJumping true)
  (Components|Timeline|SetPlayRate (Variables|Default|GetDoJumpTimeline) (Variables|Default|GetJumpSpeed))
  (Audio|PlaySound2D "/Game/Audio/Hop.Hop")
  (bind _jump_height (Timeline|DoJumpTimeline Play)
    (:Update
      (Variables|Default|SetJumpHeight (* (Transformation|GetActorUpVector) _jump_height)))
    (:Finished
      (Variables|Default|SetIsJumping false))))

(event Custom|Fork
  ;[1 1 1] Fork
  (bind _asfork_trigger (Utilities|Casting|CastToForkTrigger (Variables|Default|GetCollision)))
  (bind _outactors (Actor|GetAllActorsOfClass "/Game/Blueprints/TrackManager.TrackManager_C"))
  (for _array_element _outactors
    (bind _result (Math|Integer|IncrementInt (Variables|/Game/Blueprints/TrackManager.TrackManager_C|GetCurrindex _array_element))
      (:%20%20
        (for (_array_element_2 _array_index) (Variables|/Game/Blueprints/TrackManager.TrackManager_C|GetSplineList _array_element)
          (bind _astrack_gen_v1 (Utilities|Casting|CastToTrackGenV1 _array_element_2))
          (if (== (Variables|/Game/Blueprints/TrackGenV1.TrackGenV1_C|GetIndex _astrack_gen_v1) (Variables|/Game/Blueprints/ForkTrigger.ForkTrigger_C|GetTrackIndexConnection _asfork_trigger))
            (if (not (>= _result (Utilities|Array|Length (Variables|/Game/Blueprints/TrackManager.TrackManager_C|GetSplineList _array_element))))
              (bind _outactors_2 (Actor|GetAllActorsOfClass "Character_Blueprint_C"))
              (for _array_element_3 _outactors_2
                _)
              (Variables|Character_Blueprint_C|SetSplineBP _array_element_3 (Utilities|Array|Get(acopy) (Variables|/Game/Blueprints/TrackManager.TrackManager_C|GetSplineList _array_element) _array_index))
              (Development|PrintString (Utilities|GetObjectName (Utilities|Array|Get(acopy) (Variables|/Game/Blueprints/TrackManager.TrackManager_C|GetSplineList _array_element) _array_index)))
              (Variables|Default|SetDistance%20Along%20Spline 0.0)
              (bind _outactors_3 (Actor|GetAllActorsOfClass "/Game/Blueprints/TrackManager.TrackManager_C"))
              (for _array_element_4 _outactors_3
                (bind _output_get (Variables|/Game/Blueprints/TrackManager.TrackManager_C|SetCurrindex _array_element_4 (Variables|/Game/Blueprints/TrackGenV1.TrackGenV1_C|GetIndex (Variables|Default|GetSplineBP))))
                (Development|PrintString (Utilities|String|ToString(Integer) _output_get))))))))))

(event Custom|Tick2
  ;[1 1 1] Movement Using Arrow Keys (For Testing)
  (Utilities|FlowControl|Gate true
    (:Exit
      (Math|Float|CompareFloat (Variables|Default|GetWidth%20Along%20Spline) -5.5e+02
        (:>
          (Variables|Default|SetWidth%20Along%20Spline (+ (Variables|Default|GetWidth%20Along%20Spline) -3e+01))
          (Transformation|SetActorLocation (+ (Transformation|GetActorLocation) (* (Variables|Default|GetSpline%20Tangent) -3e+01)) false false))))))

(event Custom|Tick1
  ;[1 1 1] Movement Using Arrow Keys (For Testing)
  (Utilities|FlowControl|Gate true
    (:Exit
      (Math|Float|CompareFloat (Variables|Default|GetWidth%20Along%20Spline) 5.5e+02
        (:<
          (Variables|Default|SetWidth%20Along%20Spline (+ (Variables|Default|GetWidth%20Along%20Spline) 3e+01))
          (Transformation|SetActorLocation (+ (* (Variables|Default|GetSpline%20Tangent) 3e+01) (Transformation|GetActorLocation)) false false))))))

(event Collision|EventActorBeginOverlap
  (params (OtherActor :type Actor%20Object%20Reference))
  (bind _returnvalue (Utilities|GetClass OtherActor))
  ;[1 1 1] Collecting Items
  (Variables|Default|SetCollision OtherActor)
  (if (Utilities|ClassIsChildOf _returnvalue "/Game/Blueprints/Collectible_Blueprint.Collectible_Blueprint_C")
    (if (Variables|Default|GetCreateMode)
      (Actor|DestroyActor OtherActor)
      (Effects|SpawnEmitteratLocation "/Game/InfinityBladeEffects/Effects/FX_Monsters/FX_Monster_Gruntling/Bomber/P_FireBombExplosion.P_FireBombExplosion" (Transformation|GetActorLocation))
      (Audio|PlaySound2D "/Game/Audio/Jab.Jab")
      (Variables|Default|SetCollected (+ (Variables|Default|GetCollected) (* 1 (Variables|Default|GetMultiplier)))))
    (else
      ;[1 1 1] Ramps
      (if (Utilities|ClassIsChildOf _returnvalue "/Game/Blueprints/Ramp_Blueprint.Ramp_Blueprint_C")
        (CallFunction|DoJump)
        (elif (Utilities|ClassIsChildOf _returnvalue "/Game/Blueprints/ForkTrigger.ForkTrigger_C")
          (CallFunction|Fork))))))

(event EventTick
  (params (DeltaSeconds :type Float%20%28single-precision%29))
  (bind _self self)
  ;[1 1 1] Take Character and Apply Input
  (CallFunction|Tick3)
  (if (Variables|Default|GetMove)
    (Variables|/Script/Engine.PlayerController|SetbShowMouseCursor (Game|GetPlayerController 0) true)
    (Variables|Default|SetDistance%20Along%20Spline (+ (* (Math|Float|MakeLiteralFloat (Variables|Default|GetCharacterForwardMovementSpeed)) (Utilities|Time|GetWorldDeltaSeconds)) (Variables|Default|GetDistance%20Along%20Spline)))
    ;[1 1 1] Apply Results of Clamp Range & Rotation from Spline
    (if (Variables|Default|GetIsJumping)
      (Variables|Default|SetCurrent%20Position (+ (Spline|GetLocationatDistanceAlongSpline (Variables|/Game/Blueprints/TrackGenV1.TrackGenV1_C|GetSpline (Variables|Default|GetSplineBP)) (Variables|Default|GetDistance%20Along%20Spline) "World") (Variables|Default|GetJumpHeight)))
      (else
        (Variables|Default|SetCurrent%20Position (Spline|GetLocationatDistanceAlongSpline (Variables|/Game/Blueprints/TrackGenV1.TrackGenV1_C|GetSpline (Variables|Default|GetSplineBP)) (Variables|Default|GetDistance%20Along%20Spline) "World"))))
    (Variables|Default|SetCurrent%20Rotation (Spline|GetRotationatDistanceAlongSpline (Variables|/Game/Blueprints/TrackGenV1.TrackGenV1_C|GetSpline (Variables|Default|GetSplineBP)) (Variables|Default|GetDistance%20Along%20Spline) "World"))
    (Transformation|SetActorLocation _self (+ (* (Transformation|GetActorRightVector) (Variables|Default|GetWidth%20Along%20Spline)) (Variables|Default|GetCurrent%20Position)) false false)
    (Transformation|SetActorRotation _self (Spline|GetRotationatDistanceAlongSpline (Variables|/Game/Blueprints/TrackGenV1.TrackGenV1_C|GetSpline (Variables|Default|GetSplineBP)) (Variables|Default|GetDistance%20Along%20Spline) "World"))
    (Variables|Default|SetSpline%20Tangent (Math|Vector|GetRightVector (Math|Conversions|RotationFromXVector (Math|Vector|GetForwardVector (Math|Conversions|RotationFromXVector (Spline|GetTangentatDistanceAlongSpline (Variables|/Game/Blueprints/TrackGenV1.TrackGenV1_C|GetSpline (Variables|Default|GetSplineBP)) (Variables|Default|GetDistance%20Along%20Spline) "Local"))))))
    (CallFunction|Tick1)
    (CallFunction|Tick2)
    ;[1 1 1] Moving On To Next Spline
    (CallFunction|Tick4)
    (Variables|Default|SetTotalLength (Spline|GetDistanceAlongSplineatSplinePoint (Variables|/Game/Blueprints/TrackGenV1.TrackGenV1_C|GetSpline (Variables|Default|GetSplineBP)) (- (Spline|GetNumberOfSplinePoints (Variables|/Game/Blueprints/TrackGenV1.TrackGenV1_C|GetSpline (Variables|Default|GetSplineBP))) 1)))
    (if (>= (Variables|Default|GetDistance%20Along%20Spline) (Spline|GetDistanceAlongSplineatSplinePoint (Variables|/Game/Blueprints/TrackGenV1.TrackGenV1_C|GetSpline (Variables|Default|GetSplineBP)) (- (Spline|GetNumberOfSplinePoints (Variables|/Game/Blueprints/TrackGenV1.TrackGenV1_C|GetSpline (Variables|Default|GetSplineBP))) 1)))
      (if (not (== (Variables|/Game/Blueprints/TrackGenV1.TrackGenV1_C|GetNextIndex (Variables|Default|GetSplineBP)) -1))
        (if (== (Variables|/Game/Blueprints/TrackGenV1.TrackGenV1_C|GetNextIndex (Variables|Default|GetSplineBP)) 0)
          (bind _outactors (Actor|GetAllActorsOfClass "/Game/Blueprints/TrackManager.TrackManager_C"))
          (for _array_element _outactors
            (bind _result (Math|Integer|IncrementInt (Variables|/Game/Blueprints/TrackManager.TrackManager_C|GetCurrindex _array_element))
              (:%20%20
                (for (_array_element_2 _array_index) (Variables|/Game/Blueprints/TrackManager.TrackManager_C|GetSplineList _array_element)
                  (if (== (Variables|/Game/Blueprints/TrackGenV1.TrackGenV1_C|GetIndex _array_element_2) _result)
                    (bind _outactors_2 (Actor|GetAllActorsOfClass "Character_Blueprint_C"))
                    (for _array_element_3 _outactors_2
                      _)
                    (Variables|Character_Blueprint_C|SetSplineBP _array_element_3 (Utilities|Array|Get(acopy) (Variables|/Game/Blueprints/TrackManager.TrackManager_C|GetSplineList _array_element) _array_index))
                    (Development|PrintString (Utilities|GetObjectName (Utilities|Array|Get(acopy) (Variables|/Game/Blueprints/TrackManager.TrackManager_C|GetSplineList _array_element) _array_index)))
                    (Variables|Default|SetDistance%20Along%20Spline 0.0)
                    (bind _outactors_3 (Actor|GetAllActorsOfClass "/Game/Blueprints/TrackManager.TrackManager_C"))
                    (for _array_element_4 _outactors_3
                      (bind _output_get (Variables|/Game/Blueprints/TrackManager.TrackManager_C|SetCurrindex _array_element_4 (Variables|/Game/Blueprints/TrackGenV1.TrackGenV1_C|GetIndex (Variables|Default|GetSplineBP))))
                      (Development|PrintString (Utilities|String|ToString(Integer) _output_get))))))))
          (else
            (bind _outactors_4 (Actor|GetAllActorsOfClass "/Game/Blueprints/TrackManager.TrackManager_C"))
            (for _array_element_5 _outactors_4
              (for (_array_element_6 _array_index_2) (Variables|/Game/Blueprints/TrackManager.TrackManager_C|GetSplineList _array_element_5)
                (if (== (Variables|/Game/Blueprints/TrackGenV1.TrackGenV1_C|GetIndex _array_element_6) (Variables|/Game/Blueprints/TrackGenV1.TrackGenV1_C|GetNextIndex (Variables|Default|GetSplineBP)))
                  (bind _outactors_5 (Actor|GetAllActorsOfClass "Character_Blueprint_C"))
                  (for _array_element_7 _outactors_5
                    _)
                  (Variables|Character_Blueprint_C|SetSplineBP _array_element_7 (Utilities|Array|Get(acopy) (Variables|/Game/Blueprints/TrackManager.TrackManager_C|GetSplineList _array_element_5) _array_index_2))
                  (Development|PrintString (Utilities|GetObjectName (Utilities|Array|Get(acopy) (Variables|/Game/Blueprints/TrackManager.TrackManager_C|GetSplineList _array_element_5) _array_index_2)))
                  (Variables|Default|SetDistance%20Along%20Spline 0.0)
                  (bind _outactors_6 (Actor|GetAllActorsOfClass "/Game/Blueprints/TrackManager.TrackManager_C"))
                  (for _array_element_8 _outactors_6
                    (bind _output_get_2 (Variables|/Game/Blueprints/TrackManager.TrackManager_C|SetCurrindex _array_element_8 (Variables|/Game/Blueprints/TrackGenV1.TrackGenV1_C|GetIndex (Variables|Default|GetSplineBP))))
                    (Development|PrintString (Utilities|String|ToString(Integer) _output_get_2))))))))))))

(event Input|KeyboardEvents|X
  (params (Key :type Key%20Structure :default "AnyKey"))
  ;[1 1 1] Creative Mode
  (:Pressed
    (if (Variables|Default|GetCreateMode)
      (Variables|Default|SetCreateMode false)
      (Development|PrintString "Creative Mode Enabled")
      (else
        (Variables|Default|SetCreateMode true)
        (Development|PrintString "Creative Mode Disabled")))))

(event Input|KeyboardEvents|D
  (params (Key :type Key%20Structure :default "AnyKey"))
  ;[1 1 1] Movement Using Arrow Keys (For Testing)
  (:Pressed
    (Utilities|FlowControl|Gate true) ; enters at Open
  )
  (:Released
    (Utilities|FlowControl|Gate true) ; enters at Close
  ))

(event Input|KeyboardEvents|A
  (params (Key :type Key%20Structure :default "AnyKey"))
  ;[1 1 1] Movement Using Arrow Keys (For Testing)
  (:Pressed
    (Utilities|FlowControl|Gate true) ; enters at Open
  )
  (:Released
    (Utilities|FlowControl|Gate true) ; enters at Close
  ))

(event Input|KeyboardEvents|P
  (params (Key :type Key%20Structure :default "AnyKey"))
  (bind _returnvalue (Game|GetPlayerController 0))
  ;[1 1 1] Pause
  (:Pressed
    (if (Game|IsGamePaused)
      (Game|SetGamePaused false)
      (Variables|/Script/Engine.PlayerController|SetbShowMouseCursor _returnvalue false)
      (Widget|RemovefromParent (stale _returnvalue_2))
      (else
        (Game|SetGamePaused true)
        (Variables|/Script/Engine.PlayerController|SetbShowMouseCursor _returnvalue true)
        (bind _returnvalue_2 (UserInterface|CreateWidget "/Game/Menus/PauseMenu.PauseMenu_C" _returnvalue))
        (UserInterface|Viewport|AddtoViewport _returnvalue_2 0)))))

(event Input|KeyboardEvents|SpaceBar
  (params (Key :type Key%20Structure :default "AnyKey"))
  ;[1 1 1] Creative Mode
  (:Pressed
    (bind _outactors (Actor|GetAllActorsOfClass "Character_Blueprint_C"))
    (for _array_element _outactors
      (Game|SpawnActorfromClass "/Game/Blueprints/Collectible_Blueprint.Collectible_Blueprint_C" (Math|Transform|MakeTransform (+ (.Location (Math|Transform|BreakTransform (Transformation|GetActorTransform _array_element))) (* (Transformation|GetActorUpVector _array_element) 8e+01)) (.Rotation (Math|Transform|BreakTransform (Transformation|GetActorTransform _array_element))) (.Scale (Math|Transform|BreakTransform (Transformation|GetActorTransform _array_element)))) "Undefined" 0 0))))

(event Input|TouchEvents|InputTouch
  (params (Location :type Vector) (FingerIndex :type ETouchIndex%20Enum))
  (bind _x (Math|Vector|BreakVector Location))
  (bind _returnvalue (Utilities|Time|GetWorldDeltaSeconds))
  (bind _returnvalue_2 (Game|GetPlayerController 0))
  (bind _spline_tangent (Variables|Default|GetSpline%20Tangent))
  (bind _sizex (HUD|GetViewportSize _returnvalue_2))
  (bind _returnvalue_3 (Math|Conversions|ToFloat(Integer) _sizex))
  (bind _returnvalue_4 (/ _returnvalue_3 2.0))
  ;[1 1 1] Test Touch Input
  (:Pressed
    (Variables|Default|SetCanMove true))
  (:Released
    (Variables|Default|SetCanMove false))
  (:Moved
    (if (Variables|Default|GetCanMove)
      (Variables|Default|SetMiddlePoint _returnvalue_4)
      (Variables|Default|SetFingerXPos _x)
      (Variables|Default|SetResult (* (- (Variables|Default|GetFingerXPos) (Variables|Default|GetMiddlePoint)) (Variables|Default|GetCharacterSideMovementSpeed)))
      (Math|Float|CompareFloat _x _returnvalue_4
        (:>
          (Math|Float|CompareFloat (Variables|Default|GetWidth%20Along%20Spline) 7e+02
            (:<
              (Variables|Default|SetWidth%20Along%20Spline (+ (Variables|Default|GetWidth%20Along%20Spline) (* (Variables|Default|GetResult) (Utilities|Time|GetWorldDeltaSeconds))))
              (Transformation|SetActorLocation (+ (* _spline_tangent (* _returnvalue (Variables|Default|GetResult))) (Transformation|GetActorLocation)) false false))))
        (:<
          (Math|Float|CompareFloat (Variables|Default|GetWidth%20Along%20Spline) -7e+02
            (:>
              (Variables|Default|SetWidth%20Along%20Spline (+ (Variables|Default|GetWidth%20Along%20Spline) (* (Variables|Default|GetResult) (Utilities|Time|GetWorldDeltaSeconds))))
              (Transformation|SetActorLocation (+ (Transformation|GetActorLocation) (* _spline_tangent (* (Variables|Default|GetResult) _returnvalue))) false false))))))))

(fn ConstructionScript)