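; SplineBounds actor that travels along a referenced SplineBP's spline at constant speed, acting as a movement boundary around the path.
; Each Tick advances a distance value by delta time, clamps the actor's world X, Y and Z around that spline point, and matches the spline's rotation.
; Gated A/D test input nudges it sideways along the mesh's right vector before clamping.
; All range limits are currently zero, pinning it to the spline.
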(event Custom|Tick2
  ;[1 1 1] Movement Using Arrow Keys (For Testing)
  (Utilities|FlowControl|Gate true
    (:Exit
      (Transformation|SetActorLocation (+ (Transformation|GetActorLocation) (* (Math|Vector|GetRightVector (Variables|Default|GetSplineBounds_StaticMesh)) -3e+01)) false false))))

(event Custom|Tick1
  ;[1 1 1] Movement Using Arrow Keys (For Testing)
  (Utilities|FlowControl|Gate true
    (:Exit
      (Transformation|SetActorLocation (+ (* (Math|Vector|GetRightVector (Variables|Default|GetSplineBounds_StaticMesh)) 3e+01) (Transformation|GetActorLocation)) false false))))

(event EventTick
  (params (DeltaSeconds :type Float%20%28single-precision%29))
  (bind _returnvalue (Math|Float|MakeLiteralFloat 0.0))
  (bind _returnvalue_2 (Math|Float|MakeLiteralFloat 0.0))
  (bind _returnvalue_3 (Math|Float|MakeLiteralFloat 0.0))
  (bind _returnvalue_4 (Transformation|GetActorLocation))
  (bind _self self)
  (bind (_x _y _z) (Math|Vector|BreakVector _returnvalue_4))
  ;[1 1 1] Take Character and Apply Input
  (CallFunction|Tick1)
  (CallFunction|Tick2)
  (Variables|Default|SetPosition (+ (* (Math|Float|MakeLiteralFloat 2e+03) (Utilities|Time|GetWorldDeltaSeconds)) (Variables|Default|GetPosition)))
  ;[1 1 1] Apply Results of Clamp Range & Rotation from Spline
  (Transformation|SetActorLocation _self (Math|Vector|MakeVector (Math|Float|Clamp(Float) _x (+ (.X (Math|Vector|BreakVector (Spline|GetLocationatDistanceAlongSpline (Variables|/Game/Blueprints/SplineBP.SplineBP_C|GetSpline (Variables|Default|GetSplineBP)) (Variables|Default|GetPosition) "World"))) (* _returnvalue_2 -1.0)) (+ (.X (Math|Vector|BreakVector (Spline|GetLocationatDistanceAlongSpline (Variables|/Game/Blueprints/SplineBP.SplineBP_C|GetSpline (Variables|Default|GetSplineBP)) (Variables|Default|GetPosition) "World"))) _returnvalue_2)) (Math|Float|Clamp(Float) _y (+ (.Y (Math|Vector|BreakVector (Spline|GetLocationatDistanceAlongSpline (Variables|/Game/Blueprints/SplineBP.SplineBP_C|GetSpline (Variables|Default|GetSplineBP)) (Variables|Default|GetPosition) "World"))) (* _returnvalue_3 -1.0)) (+ (.Y (Math|Vector|BreakVector (Spline|GetLocationatDistanceAlongSpline (Variables|/Game/Blueprints/SplineBP.SplineBP_C|GetSpline (Variables|Default|GetSplineBP)) (Variables|Default|GetPosition) "World"))) _returnvalue_3)) (Math|Float|Clamp(Float) _z (+ (.Z (Math|Vector|BreakVector (Spline|GetLocationatDistanceAlongSpline (Variables|/Game/Blueprints/SplineBP.SplineBP_C|GetSpline (Variables|Default|GetSplineBP)) (Variables|Default|GetPosition) "World"))) _returnvalue) (+ (.Z (Math|Vector|BreakVector (Spline|GetLocationatDistanceAlongSpline (Variables|/Game/Blueprints/SplineBP.SplineBP_C|GetSpline (Variables|Default|GetSplineBP)) (Variables|Default|GetPosition) "World"))) _returnvalue))) false false)
  (Transformation|SetActorRotation _self (Spline|GetRotationatDistanceAlongSpline (Variables|/Game/Blueprints/SplineBP.SplineBP_C|GetSpline (Variables|Default|GetSplineBP)) (Variables|Default|GetPosition) "World")))

(event Input|KeyboardEvents|A
  (params (Key :type Key%20Structure :default "AnyKey"))
  ;[1 1 1] Movement Using Arrow Keys (For Testing)
  (:Pressed
    (Utilities|FlowControl|Gate true) ; enters at Open
  )
  (:Released
    (Utilities|FlowControl|Gate true) ; enters at Close
  ))

(event Input|KeyboardEvents|D
  (params (Key :type Key%20Structure :default "AnyKey"))
  ;[1 1 1] Movement Using Arrow Keys (For Testing)
  (:Pressed
    (Utilities|FlowControl|Gate true) ; enters at Open
  )
  (:Released
    (Utilities|FlowControl|Gate true) ; enters at Close
  ))

(fn ConstructionScript)