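; Track generator actor that lays highway road meshes along its spline in the construction script.
; It adds a spline mesh per spacing interval, swapping to a second road mesh at a set alternating rate and applying cull distance.
; Segment ends take world-space position, scaled direction tangents and roll from the spline, so the road follows banking.
; The event graph does nothing at runtime, holding only unconnected lookup nodes.
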(event EventBeginPlay)

(event Collision|EventActorBeginOverlap
  (params (OtherActor :type Actor%20Object%20Reference)))

(event EventTick
  (params (DeltaSeconds :type Float%20%28single-precision%29)))

(fn ConstructionScript
  (bind _tangentscale (Variables|Default|GetTangentScale))
  (bind _spline (Variables|Default|GetSpline))
  (bind _spacing (Variables|Default|GetSpacing))
  (for _index (range 0 (.ReturnValue (Math|Float|Division(WholeandRemainder) (Spline|GetSplineLength (Variables|Default|GetSpline)) _spacing)))
    (bind _returnvalue (AddComponent|AddSplineMeshComponent true))
    (bind _result (Math|Integer|IncrementInt (Variables|Default|GetMeshCounter))
      (:%20%20
        (if (== (Math|Integer|%(Integer) _result (Variables|Default|GetAlternatingRate)) 0)
          (Components|StaticMesh|SetStaticMesh _returnvalue "/Game/Meshes/High_way_road2.High_way_road2")
          (else
            (Components|StaticMesh|SetStaticMesh _returnvalue "/Game/Meshes/High_way_road.High_way_road")))
        (Class|PrimitiveComponent|SetCullDistance _returnvalue 2e+04)
        (SplineMesh|SetStartandEnd _returnvalue (Spline|GetLocationatDistanceAlongSpline _spline (* _index _spacing) "World") (* (Spline|GetDirectionatDistanceAlongSpline _spline (* _index _spacing) "World") _tangentscale) (Spline|GetLocationatDistanceAlongSpline _spline (+ (* _index _spacing) (Variables|Default|GetSpacing)) "World") (* (Spline|GetDirectionatDistanceAlongSpline _spline (+ (* _index _spacing) (Variables|Default|GetSpacing)) "World") _tangentscale) true :!class /Script/Engine.SplineMeshComponent)
        (Class|SplineMeshComponent|SetStartRoll _returnvalue (Math|Trig|DegreesToRadians (.Roll (Math|Rotator|BreakRotator (Spline|GetRotationatDistanceAlongSpline _spline (* _index _spacing) "World")))) true)
        (Class|SplineMeshComponent|SetEndRoll _returnvalue (Math|Trig|DegreesToRadians (.Roll (Math|Rotator|BreakRotator (Spline|GetRotationatDistanceAlongSpline _spline (+ (* _index _spacing) (Variables|Default|GetSpacing)) "World")))) true)))))