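; TrackManager orders the level's TrackGenV1 track actors and hands one to the player character Blueprint as its spline reference.
; The construction script gathers those actors into SplineList and bubble-sorts them by Index, printing debug strings.
; On BeginPlay it loops over Character_Blueprint actors with an empty body, then sets SplineBP on the last element to the entry just before Currindex.
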(event EventBeginPlay
  (bind _outactors (Actor|GetAllActorsOfClass "/Game/Blueprints/Character_Blueprint.Character_Blueprint_C"))
  (for _array_element _outactors
    _)
  (Variables|/Game/Blueprints/Character_Blueprint.Character_Blueprint_C|SetSplineBP _array_element (Utilities|Array|Get(acopy) (Variables|Default|GetSplineList) (- (Variables|Default|GetCurrindex) 1))))

(event Collision|EventActorBeginOverlap
  (params (OtherActor :type Actor%20Object%20Reference)))

(event EventTick
  (params (DeltaSeconds :type Float%20%28single-precision%29)))

(fn ConstructionScript
  (bind _outactors (Actor|GetAllActorsOfClass "/Game/Blueprints/TrackGenV1.TrackGenV1_C"))
  (Variables|Default|SetSplineList _outactors)
  (for _index (range 0 (- (Utilities|Array|Length (Variables|Default|GetSplineList)) 1))
    (for _index_2 (range 0 (- (- (- (Utilities|Array|Length (Variables|Default|GetSplineList)) 1) _index) 1))
      (Variables|Default|SetIndex _index_2)
      (Variables|Default|Setlist[i] (Utilities|Array|Get(acopy) (Variables|Default|GetSplineList) _index_2))
      (Variables|Default|Setlist[i+1] (Utilities|Array|Get(acopy) (Variables|Default|GetSplineList) (+ _index_2 1)))
      (Development|PrintString (Utilities|String|ToString(Integer) (Variables|/Game/Blueprints/TrackGenV1.TrackGenV1_C|GetIndex (Utilities|Array|Get(acopy) (Variables|Default|GetSplineList) _index_2))))
      (Development|PrintString (Utilities|String|ToString(Integer) (Variables|/Game/Blueprints/TrackGenV1.TrackGenV1_C|GetIndex (Utilities|Array|Get(acopy) (Variables|Default|GetSplineList) (+ _index_2 1)))))
      (if (< (Variables|/Game/Blueprints/TrackGenV1.TrackGenV1_C|GetIndex (Utilities|Array|Get(acopy) (Variables|Default|GetSplineList) (+ _index_2 1))) (Variables|/Game/Blueprints/TrackGenV1.TrackGenV1_C|GetIndex (Utilities|Array|Get(acopy) (Variables|Default|GetSplineList) _index_2)))
        (Development|PrintString "Swapping")
        (Variables|Default|Settemp (Variables|Default|Getlist[i]))
        (bind _output_get (Variables|Default|Setlist[i] (Variables|Default|Getlist[i+1])))
        (bind _output_get_2 (Variables|Default|Setlist[i+1] (Variables|Default|Gettemp)))
        (Utilities|Array|SetArrayElem (Variables|Default|GetSplineList) (Variables|Default|GetIndex) _output_get)
        (Utilities|Array|SetArrayElem (Variables|Default|GetSplineList) (+ (Variables|Default|GetIndex) 1) _output_get_2)))))